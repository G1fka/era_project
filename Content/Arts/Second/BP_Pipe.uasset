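; BP_Pipe is a pipe actor, apparently the base for rotatable puzzle pieces, that reports whether it sits at its correct angle.
; IsConnected compares the absolute remainder of its yaw with RightAngle, returning the result plus both angles.
; It casts itself to subtypes: cross pieces always pass, straight pieces repeat every half turn, and others need a full turn.
; GetWidget exposes its widget, while the event graph and construction script are empty.
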(fn `Get Widget`
  (returns (Widget :type "WidgetComponent Object Reference"))
  (return (`self.Widget`)))

(fn `Is Connected`
  (returns (`Is Connected` :type Boolean) (`Required Angle` :type "Float (double-precision)") (`Actual Angle` :type "Float (double-precision)"))
  (bind _yaw (.yaw (`self.K2_GetActorRotation`)))
  (cast `/Game/Arts/Second/BP_Pipe_Cross` self
    (:`then`
      (return true -1.0 -1.0))
    (:`CastFailed`
      (bind _output_get (set `self.Right Angle` (`KismetMathLibrary.Abs` (`self.Right Angle`))))
      (cast `/Game/Arts/Second/BP_Pipe_Straight` self
        (:`then`
          (set `self.Divizor` 180.0)
          (if (== _output_get 180.0)
            (bind _output_get_2 (set `self.Right Angle` 0.0))))
        (:`CastFailed`
          (set `self.Divizor` 360.0)))
      (set `self.Remainder` (`KismetMathLibrary.Abs` (`KismetMathLibrary.FMod` _yaw (`self.Divizor`))))
      (return (== (`self.Right Angle`) (`self.Remainder`)) _output_get_2 _yaw))))

(fn `UserConstructionScript`)