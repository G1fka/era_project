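; BP_Handwheel is an interactable handwheel that checks whether the level's pipe puzzle is connected.
; Overlap by the first-person character sets its Overlapping ID to mark the wheel, clears it on exit, and toggles a widget's visibility each time.
; The Check event loops over all BP_Pipe actors, stops at the first disconnected one, and prints success or error.
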(event `self.ReceiveActorEndOverlap`
  (params (OtherActor :type "Actor Object Reference"))
  (bind _widget (`self.Widget`))
  (bind _asbp_first_person_character (cast `/Game/FirstPerson/Blueprints/BP_FirstPersonCharacter` OtherActor))
  (set `/Game/FirstPerson/Blueprints/BP_FirstPersonCharacter.Overlapping` -1 _asbp_first_person_character)
  (`SceneComponent.SetVisibility` _widget (not (`WidgetComponent.IsWidgetVisible` _widget)) false :!label _label))

(event `self.ReceiveActorBeginOverlap`
  (params (OtherActor :type "Actor Object Reference"))
  (bind _asbp_first_person_character (cast `/Game/FirstPerson/Blueprints/BP_FirstPersonCharacter` OtherActor))
  (set `/Game/FirstPerson/Blueprints/BP_FirstPersonCharacter.Overlapping` 4 _asbp_first_person_character)
  (goto _label))

(event `/Game/Arts/Second/BPI_Check.Check`
  (bind _outactors (`GameplayStatics.GetAllActorsOfClass` "/Game/Arts/Second/BP_Pipe.BP_Pipe_C"))
  (for _array_element _outactors
    (bind _is_connected (`/Game/Arts/Second/BP_Pipe.Is Connected` _array_element))
    (if (not _is_connected)
      (break)))
  (if _is_connected
    (`KismetSystemLibrary.PrintString` "Success")
    (else
      (`KismetSystemLibrary.PrintString` "Error"))))

(fn `UserConstructionScript`)